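; Bomb projectile that explodes on players other than its owner and stuns the car pawn it hits.
; A sphere overlap sized from ExplosionRadius at construction detects targets, and only the authority triggers the explosion and stun.
; A missile sound attaches on BeginPlay.
; The OnExplosion event handles cosmetics, destroying the missile effect component and spawning a scaled particle burst and blast sound.
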(event OnComponentBeginOverlap(overlap)
  (params (OverlappedComponent :type Primitive%20Component%20Object%20Reference) (OtherActor :type Actor%20Object%20Reference) (OtherComp :type Primitive%20Component%20Object%20Reference) (OtherBodyIndex :type Integer) (bFromSweep :type Boolean) (SweepResult :type Hit%20Result%20Structure%20%28by%20ref%29))
  (Networking|SwitchHasAuthority
    (:Authority
      (if (and (Actor|ActorHasTag OtherActor "Player") (!= OtherActor (Components|GetOwner)))
        (Class|BombProjectile|Explosion)
        (bind _ascar_pawn (Utilities|Casting|CastToCarPawn OtherActor))
        (Class|CarPawn|Stan _ascar_pawn (Variables|Default|GetStanTime))))))

(event EventBeginPlay
  (Audio|SpawnSoundAttached "/Game/Assets/Sound/Cue_MissleEffect.Cue_MissleEffect" (Variables|Default|GetCollisionComponent) "None" "0, 0, 0" "0, 0, 0" "SnapToTarget" false 1.0 1.0 0.0 0 0))

(event Collision|EventActorBeginOverlap
  (params (OtherActor :type Actor%20Object%20Reference)))

(event EventTick
  (params (DeltaSeconds :type Float%20%28single-precision%29)))

(event EventOnExplosion
  (bind _returnvalue (Transformation|GetActorLocation))
  (Components|DestroyComponent (Variables|Default|GetCue_MissleEffect))
  (Effects|SpawnEmitteratLocation "/Game/Assets/Realistic_Starter_VFX_Pack_Vol2/Particles/Explosion/P_Explosion_Big_B.P_Explosion_Big_B" _returnvalue "0, 0, 0" (Math|Conversions|ToVector(Float) (/ (Variables|Default|GetParticleScale) 5e+01)))
  (Audio|PlaySoundatLocation "/Game/Assets/Sound/587194__derplayer__explosion-big-01.587194__derplayer__explosion-big-01" _returnvalue "0, 0, 0" 1.0 1.0 0.0 0 0 0 0))

(fn ConstructionScript
  (Components|Sphere|SetSphereRadius (Variables|Default|Getoverlap) (Variables|Default|GetExplosionRadius) true))